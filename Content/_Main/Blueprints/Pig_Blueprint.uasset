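; Pig actor with a skeletal mesh that can switch to ragdoll physics, expose its tail-tip socket location and change to a roasted look.
; Ragdoll on BeginPlay is disabled, and hits from other pigs fire a dispatcher.
; Any change in roasted state creates a dynamic material tinted with the roasted color, even when un-roasting.
; The tail-tip constraint function is an empty stub with its constraint logic unconnected.
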(event `self.ReceiveBeginPlay`
  (`self.Go Ragdoll` :!enabledstate Disabled))

(event `self.ReceiveHit`
  (params (MyComp :type "PrimitiveComponent Object Reference") (Other :type "Actor Object Reference") (OtherComp :type "PrimitiveComponent Object Reference") (bSelfMoved :type Boolean) (HitLocation :type "Vector Structure") (HitNormal :type "Vector Structure") (NormalImpulse :type "Vector Structure") (Hit :type "HitResult Structure (by ref)"))
  (cast `/Game/_Main/Blueprints/Pig_Blueprint` Other)
  (`self.Hit By Other Pig Blueprint Actor`))

(event `self.ReceiveTick`
  (params (DeltaSeconds :type "Float (single-precision)")))

(fn `Get Tail Tip Location`
  (returns (`World Location` :type "Vector Structure"))
  (return (`SceneComponent.GetSocketLocation` (`self.SkeletalMeshComponent0`) "PIG_-Tail-socket")))

(fn `Go Ragdoll`
  (`PrimitiveComponent.SetSimulatePhysics` (`self.GetComponentByClass` self "/Script/Engine.SkeletalMeshComponent") true))

(fn `Set Constraint Component To Tail Tip`
  (params (`Phys Constraint Component` :type "PhysicsConstraintComponent Object Reference") (`Grab Point Component` :type "PrimitiveComponent Object Reference")))

(fn `Set Is Roasted`
  (params (Roasted :type Boolean))
  (if (xor Roasted (`self.Is Roasted`))
    (set `self.Is Roasted` Roasted)
    (bind _returnvalue (`PrimitiveComponent.CreateDynamicMaterialInstance` (`self.SkeletalMeshComponent0`) 0 "/Game/FarmAnimalsPack/Pig/Materials/M_Pig.M_Pig" "None"))
    (`MaterialInstanceDynamic.SetVectorParameterValue` _returnvalue "Base Color Multiply" (`self.Roasted Color`))))

(fn `UserConstructionScript`)