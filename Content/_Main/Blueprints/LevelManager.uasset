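; Level manager Blueprint that completes a level once both left and right pig triggers have reported a roasted pig, then advances to the next.
; It binds to each trigger's pig overlap event and latches a flag per side; when both are set, it shows completion text and, after delays, opens the named next level if set.
; It also provides functions to restart the current level and spawn randomly rotated pigs with configurable grabbed and roasted states.
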(event `self.ReceiveBeginPlay`
  (add `/Game/_Main/Blueprints/PigTrigger.Pig Overlap` (`self.Pig Trigger L`) (delegate `Nose L In Pig`))
  (add `/Game/_Main/Blueprints/PigTrigger.Pig Overlap` (`self.Pig Trigger R`) (delegate `Nose R In Pig`)))

(event `Nose L In Pig`
  (params (`Target Pig Blueprint` :type "/Game/_Main/Blueprints/Pig_Blueprint Object Reference"))
  (if (`/Game/_Main/Blueprints/Pig_Blueprint.Is Roasted` `Target Pig Blueprint`)
    (set `self.L OK` true)
    (`self.Check Level Complete` :!label _label)))

(event `Nose R In Pig`
  (params (`Target Pig Blueprint` :type "/Game/_Main/Blueprints/Pig_Blueprint Object Reference"))
  (if (`/Game/_Main/Blueprints/Pig_Blueprint.Is Roasted` `Target Pig Blueprint`)
    (set `self.R OK` true)
    (goto _label)))

(event `Check Level Complete`
  (if (and (`self.L OK`) (`self.R OK`))
    (`KismetSystemLibrary.Delay` 1.0)
    (`self.On Complete Level`)))

(event `On Complete Level`
  (`TextRenderComponent.K2_SetText` (`TextRenderActor.TextRender` (`self.Level Text Render`)) (`self.Level Complete Text`))
  (`KismetSystemLibrary.Delay` 2.0)
  (`self.Go Next Level`))

(fn `Go Next Level`
  (bind _next_level_name (`self.Next Level Name`))
  (if (`self.Has Next Level`)
    (`GameplayStatics.OpenLevel` _next_level_name)
    (`KismetSystemLibrary.PrintString` (`KismetStringLibrary.Concat_StrStr` "To Level: " (`KismetStringLibrary.Conv_NameToString` _next_level_name)))))

(fn `Has Next Level`
  (returns (Result :type Boolean))
  (return (!= (`self.Next Level Name`) "None")))

(fn `Restart Level`
  (bind _returnvalue (`GameplayStatics.GetCurrentLevelName` true))
  (`GameplayStatics.OpenLevel` (`KismetStringLibrary.Conv_StringToName` _returnvalue)))

(fn `Spawn Pig`
  (params (Location :type "Vector Structure") (`Is Grabbed` :type Boolean))
  (bind _returnvalue (`|SpawnActorFromClass` (`self.Pig Class`) (`KismetMathLibrary.MakeTransform` Location (`KismetMathLibrary.RandomRotator` false)) "Undefined" "MultiplyWithRoot" null null))
  (`/Game/_Main/Blueprints/Pig.Set Grabbing` _returnvalue `Is Grabbed` false)
  (`/Game/_Main/Blueprints/Pig.Set Roasted` _returnvalue (`self.Will Spawn Roasted`)))

(fn `UserConstructionScript`)