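; An actor that defines a rectangular X/Y area, named as the boundary where the mouse is available.
; Its IsInBroundary function reports whether a given location lies within the min and max X and Y bounds, ignoring Z.
; The construction script can optionally set MaxX from the actor's own X position, so that edge follows its placement.
; The event graph holds no active logic.
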(fn `Is In Broundary`
  (params (Location :type "Vector Structure"))
  (returns (Result :type Boolean))
  (return (and (`KismetMathLibrary.InRange_FloatFloat` (.x Location) (`self.Min X`) (`self.Max X`)) (`KismetMathLibrary.InRange_FloatFloat` (.y Location) (`self.Min Y`) (`self.Max Y`)))))

(fn `UserConstructionScript`
  (if (`self.Max X Same As Self X`)
    (set `self.Max X` (.x (`self.K2_GetActorLocation`)))))