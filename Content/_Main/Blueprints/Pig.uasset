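; Pig actor that wraps a Pig_Blueprint in a child actor component and can create a physics constraint at its tail tip.
; The construction script casts and caches that child actor, printing whether the cast succeeds.
; GenerateTailTipConstraint adds a constraint component at the child's tail tip location, passes it to the child to set up on the tail tip, and returns it.
; The event graph holds no logic.
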(event `self.ReceiveBeginPlay`)

(fn `Generate Tail Tip Constraint`
  (returns (Generated :type "PhysicsConstraintComponent Object Reference"))
  (bind _child_pig_blueprint (`self.Child Pig Blueprint`))
  (bind _returnvalue (`AddComponent|NODE_AddPhysicsConstraintComponent-0`))
  (`SceneComponent.K2_SetWorldLocation` _returnvalue (`/Game/_Main/Blueprints/Pig_Blueprint.Get Tail Tip Location` _child_pig_blueprint) false true)
  (`/Game/_Main/Blueprints/Pig_Blueprint.Set Constraint Component To Tail Tip` _child_pig_blueprint _returnvalue)
  (return _returnvalue))

(fn `UserConstructionScript`
  (bind _aspig_blueprint (cast `/Game/_Main/Blueprints/Pig_Blueprint` (`ChildActorComponent.ChildActor` (`self.Pig_Blueprint`)))
    (:`then`
      (set `self.Child Pig Blueprint` _aspig_blueprint)
      (`KismetSystemLibrary.PrintString` "cast child pig blueprint suceed"))
    (:`CastFailed`
      (`KismetSystemLibrary.PrintString` "cast child pig blueprint failed!!!"))))